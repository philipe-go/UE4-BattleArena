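; BP_Explosion is a short-lived explosion actor that damages nearby enemies and shakes the player's camera.
; BeginPlay spawns the Niagara effect, calls CameraShake on BP_Player, then destroys the actor after a brief delay.
; Tick uses a Delay to postpone and throttle a capsule overlap query for Pawns, applying fixed damage to BP_Enemy actors through GetDamage.
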(event `self.ReceiveBeginPlay`
  (`NiagaraFunctionLibrary.SpawnSystemAtLocation` "/Game/VFX/NS_Explosion.NS_Explosion" (`self.K2_GetActorLocation`))
  (bind _asbp_player (cast `/Game/Blueprints/BP_Player` (`GameplayStatics.GetPlayerPawn` 0)))
  (`/Game/Blueprints/BP_Player.cameraShake` _asbp_player)
  (`KismetSystemLibrary.Delay` 0.5)
  (`self.K2_DestroyActor`))

(event `self.ReceiveTick`
  (params (DeltaSeconds :type "Float (single-precision)"))
  (`KismetSystemLibrary.Delay` 0.3)
  (bind _outactors (`KismetSystemLibrary.CapsuleOverlapActors` (`self.K2_GetActorLocation`) 500.0 0.0 (`|MakeArray` "ObjectTypeQuery3" :!type "EObjectTypeQuery Enum")))
  (for _array_element _outactors
    (bind _asbp_enemy (cast `/Game/Blueprints/BP_Enemy` _array_element))
    (`/Game/Blueprints/BP_Enemy.getDamage` _asbp_enemy 50)))

(fn `UserConstructionScript`)