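; BP_Sword is a sword hit actor that deals magic-rate damage to enemies it touches and then removes itself.
; On Box overlap, it calls GetDamage on a BP_Enemy, then spawns the NS_MagicCast2 Niagara effect with rolled or rotated orientation for any overlapped actor.
; It then triggers CameraShake on BP_Player and destroys itself, which only happens if that player cast succeeds.
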(event `self.Box.OnComponentBeginOverlap`
  (params (OverlappedComponent :type "PrimitiveComponent Object Reference") (OtherActor :type "Actor Object Reference") (OtherComp :type "PrimitiveComponent Object Reference") (OtherBodyIndex :type Integer) (bFromSweep :type Boolean) (SweepResult :type "HitResult Structure (by ref)"))
  (bind _asbp_enemy (cast `/Game/Blueprints/BP_Enemy` OtherActor)
    (:`then`
      (`/Game/Blueprints/BP_Enemy.getDamage` _asbp_enemy (`self.magicDamageRate`)))
    (:`CastFailed`
      _))
  (`NiagaraFunctionLibrary.SpawnSystemAtLocation` "/Game/VFX/NS_MagicCast2.NS_MagicCast2" (`self.K2_GetActorLocation`) (`KismetMathLibrary.ComposeRotators` (`self.K2_GetActorRotation`) (struct :`Yaw` 180.0)))
  (bind _asbp_player (cast `/Game/Blueprints/BP_Player` (`GameplayStatics.GetPlayerPawn` 0)))
  (`/Game/Blueprints/BP_Player.cameraShake` _asbp_player)
  (`self.K2_DestroyActor`))

(fn `UserConstructionScript`)