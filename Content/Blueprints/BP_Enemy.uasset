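; BP_Enemy is an enemy that hurts the player through touch, montage-driven melee and ranged bullet attacks.
; BeginPlay cross-links it with its health widget and the player, and Tick turns that widget toward the camera.
; Melee montage notifies toggle the damage collider, while ranged attacks spawn bullets with Niagara muzzle effects.
; GetDamage lowers HP; death requests the game mode's next enemy, drops a potion and destroys the actor.
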(event `self.ReceiveTick`
  (params (DeltaSeconds :type "Float (single-precision)"))
  ;[1 1 1] Tick - GetPotion and HP Bar
  (`|ExecutionSequence`
    (:`then_0`
      (`SceneComponent.K2_SetWorldRotation` (`self.Widget`) (`KismetMathLibrary.ComposeRotators` (`PlayerCameraManager.GetCameraRotation` (`GameplayStatics.GetPlayerCameraManager` 0)) (struct :`Yaw` 180.0)) false false))
    (:`then_1`
      (if (`self.isDead`)
        (`KismetSystemLibrary.Delay` 0.2)
        (`|SpawnActorFromClass` "/Game/Blueprints/BP_DropPotion.BP_DropPotion_C" (`KismetMathLibrary.Conv_VectorToTransform` (`self.K2_GetActorLocation`)) "Undefined" "OverrideRootScale" null null)
        (`self.K2_DestroyActor`)))))

(event `self.ReceiveBeginPlay`
  ;[1 1 1] Begin
  (`|ExecutionSequence`
    (:`then_0`
      (bind _aswbp_enemy (cast `/Game/UI/WBP_Enemy` (`WidgetComponent.GetUserWidgetObject` (`self.Widget`))))
      (set `/Game/UI/WBP_Enemy.Enemy` self _aswbp_enemy))
    (:`then_1`
      (bind _asbp_player (cast `/Game/Blueprints/BP_Player` (`GameplayStatics.GetPlayerPawn` 0)))
      (set `/Game/Blueprints/BP_Player.Enemy` self _asbp_player)
      (set `self.Player` _asbp_player))))

(event `self.ReceiveHit`
  (params (MyComp :type "PrimitiveComponent Object Reference") (Other :type "Actor Object Reference") (OtherComp :type "PrimitiveComponent Object Reference") (bSelfMoved :type Boolean) (HitLocation :type "Vector Structure") (HitNormal :type "Vector Structure") (NormalImpulse :type "Vector Structure") (Hit :type "HitResult Structure (by ref)"))
  ;[1 1 1] PlayerTouchEnemy
  (if (not (`self.isDead`))
    (bind _asbp_player (cast `/Game/Blueprints/BP_Player` Other))
    (`/Game/Blueprints/BP_Player.getDamage` _asbp_player 5)
    (`KismetSystemLibrary.Delay` 0.5)))

(event `OnLineTrace`
  (params (traceLocation :type "SceneComponent Object Reference"))
  ;[1 1 1] NOT WORKING PROPERLY - Behaviour strange
)

(event `Range`
  (params (Animation :type "AnimMontage Object Reference") (SpawnLocation :type "SceneComponent Object Reference") (SkeletalMesh :type "SkeletalMeshComponent Object Reference"))
  (bind _returnvalue (`SceneComponent.K2_GetComponentLocation` SpawnLocation))
  (bind _returnvalue_2 (`KismetMathLibrary.Conv_VectorToRotator` (`SceneComponent.GetForwardVector` SpawnLocation)))
  ;[1 1 1] RangedAttack
  (if (`self.isIdle`)
    (`|PlayMontage` SkeletalMesh Animation
      (:`then`
        (set `self.isIdle` false)
        (`|SpawnActorFromClass` "/Game/Blueprints/BP_Bullet.BP_Bullet_C" (`KismetMathLibrary.MakeTransform` _returnvalue _returnvalue_2) "Undefined" "OverrideRootScale" null null)
        (`NiagaraFunctionLibrary.SpawnSystemAtLocation` "/Game/VFX/NS_Canon1.NS_Canon1" _returnvalue _returnvalue_2))
      (:`OnCompleted`
        (set `self.isIdle` true)))))

(event `OverlapDamage`
  (params (otherActor :type "Actor Object Reference"))
  ;[1 1 1] MeleeOvelapEvents
  (bind _asbp_player (cast `/Game/Blueprints/BP_Player` otherActor)
    (:`then`
      (`/Game/Blueprints/BP_Player.getDamage` _asbp_player (`self.meleeDamageRate`))
      (set `self.attackSuccessful` false))
    (:`CastFailed`
      (set `self.attackSuccessful` true))))

(event `Melee`
  (params (skeletalMesh :type "SkeletalMeshComponent Object Reference") (animationMontage :type "AnimMontage Object Reference") (boxCollider :type "BoxComponent Object Reference"))
  ;[1 1 1] MeleeAttack
  (if (not (`/Game/Blueprints/BP_Player.isDead` (`self.Player`)))
    (bind _notifyname (`|PlayMontage` skeletalMesh animationMontage)
      (:`OnNotifyBegin`
        (switch `name` _notifyname
          (:`AttackStart`
            (`PrimitiveComponent.SetCollisionEnabled` boxCollider "QueryOnly"))
          (:`AttackEnd`
            (`PrimitiveComponent.SetCollisionEnabled` boxCollider "NoCollision")))))))

(fn `getDamage`
  (params (damageRate :type Integer))
  (bind _output_get (set `self.HP` (`KismetMathLibrary.Clamp` (- (`self.HP`) damageRate) 0 (`self.maxHP`))))
  (if (<= _output_get 0)
    (bind _asbp_spawn (cast `/Game/Blueprints/BP_Spawn` (`GameplayStatics.GetGameMode`)))
    (`/Game/Blueprints/BP_Spawn.SpawnNextEnemy` _asbp_spawn)
    (set `self.isDead` true)
    (else
      (`self.PlayAnimMontage` (`self.hitAnimation`)))))

(fn `UserConstructionScript`)