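; BP_EnemyMelee is a melee enemy Blueprint that fights with two swords, each with its own collision.
; On BeginPlay it runs the parent logic, disables both sword colliders, and sets its hit montage and health.
; Two attack events each pass a montage and one sword collider to a Melee routine.
; Overlaps on either sword call OverlapDamage on the other actor.
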(event `self.ReceiveBeginPlay`
  (`parent.ReceiveBeginPlay`)
  (`PrimitiveComponent.SetCollisionEnabled` (`self.SwordLeft`) "NoCollision")
  (`PrimitiveComponent.SetCollisionEnabled` (`self.SwordRight`) "NoCollision")
  (set `self.hitAnimation` "/Game/Animations/Enemy/Melee/AM_EnemyMelee_Hit.AM_EnemyMelee_Hit")
  (bind _output_get (set `self.maxHP` 512))
  (set `self.HP` _output_get))

(event `self.SwordLeft.OnComponentBeginOverlap`
  (params (OverlappedComponent :type "PrimitiveComponent Object Reference") (OtherActor :type "Actor Object Reference") (OtherComp :type "PrimitiveComponent Object Reference") (OtherBodyIndex :type Integer) (bFromSweep :type Boolean) (SweepResult :type "HitResult Structure (by ref)"))
  (`self.OverlapDamage` OtherActor))

(event `self.SwordRight.OnComponentBeginOverlap`
  (params (OverlappedComponent :type "PrimitiveComponent Object Reference") (OtherActor :type "Actor Object Reference") (OtherComp :type "PrimitiveComponent Object Reference") (OtherBodyIndex :type Integer) (bFromSweep :type Boolean) (SweepResult :type "HitResult Structure (by ref)"))
  (`self.OverlapDamage` OtherActor))

(event `Attack1`
  (`self.Melee` (`self.Mesh`) "/Game/Animations/Enemy/Melee/AM_EnemyMelee_Attack4.AM_EnemyMelee_Attack4" (`self.SwordLeft`)))

(event `Attack2`
  (`self.Melee` (`self.Mesh`) "/Game/Animations/Enemy/Melee/AM_EnemyMelee_Attack5.AM_EnemyMelee_Attack5" (`self.SwordRight`)))

(fn `UserConstructionScript`
  (`parent.UserConstructionScript`))