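; Blueprint for a hybrid enemy that can fire from range and punch in melee, built on parent enemy logic.
; Fire and Punch pass its montages, bullet spawn and gun collider to Range and Melee helpers; gun overlaps call OverlapDamage.
; Tick replays the death montage while dead, runs parent logic and sets rage at half health or below.
; Hit animation and line trace nodes are disconnected, noted as buggy.
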(event `self.ReceiveBeginPlay`
  (`parent.ReceiveBeginPlay`)
  (`PrimitiveComponent.SetCollisionEnabled` (`self.GunCollider`) "NoCollision")
  (bind _output_get (set `self.maxHP` 256))
  (set `self.HP` _output_get))

(event `self.ReceiveTick`
  (params (DeltaSeconds :type "Float (single-precision)"))
  (`|ExecutionSequence`
    (:`then_0`
      (if (`self.isDead`)
        (`|PlayMontage` (`self.Mesh`) "/Game/Animations/Enemy/Hybrid/AM_EnemyHybrid_Death.AM_EnemyHybrid_Death")))
    (:`then_1`
      (`parent.ReceiveTick` DeltaSeconds))
    (:`then_2`
      (if (<= (`KismetMathLibrary.Conv_IntToDouble` (`self.HP`)) (* (`KismetMathLibrary.Conv_IntToDouble` (`self.maxHP`)) 0.5))
        (set `self.isRaged` true)
        (`KismetSystemLibrary.PrintString` "Raged" true true (struct :`G` 0.66 :`B` 1.0 :`A` 1.0) 0.0)))))

(event `Fire`
  (`self.Range` "/Game/Animations/Enemy/Hybrid/AM_EnemyHybrid_Fire.AM_EnemyHybrid_Fire" (`self.BulletSpawn`) (`self.Mesh`)))

(event `Punch`
  (`self.Melee` (`self.Mesh`) "/Game/Animations/Enemy/Hybrid/AM_EnemyHybrid_Melee.AM_EnemyHybrid_Melee" (`self.GunCollider`)))

(event `self.GunCollider.OnComponentBeginOverlap`
  (params (OverlappedComponent :type "PrimitiveComponent Object Reference") (OtherActor :type "Actor Object Reference") (OtherComp :type "PrimitiveComponent Object Reference") (OtherBodyIndex :type Integer) (bFromSweep :type Boolean) (SweepResult :type "HitResult Structure (by ref)"))
  (`self.OverlapDamage` OtherActor))

(fn `UserConstructionScript`
  (`parent.UserConstructionScript`))