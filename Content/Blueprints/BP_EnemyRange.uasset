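; BP_EnemyRange is a ranged enemy Blueprint that extends parent enemy logic with its own health and firing attack.
; BeginPlay runs the parent logic, then initializes max and current HP.
; The Fire event calls Range with the ranged fire montage, bullet spawn point and mesh.
; Hit-animation assignment and line-trace logic are left disconnected, with notes that they misbehave.
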(event `self.ReceiveBeginPlay`
  (`parent.ReceiveBeginPlay`)
  (bind _output_get (set `self.maxHP` 128))
  (set `self.HP` _output_get))

(event `self.ReceiveTick`
  (params (DeltaSeconds :type "Float (single-precision)"))
  (`parent.ReceiveTick` DeltaSeconds))

(event `Fire`
  (`self.Range` "/Game/Animations/Enemy/Ranged/AM_EnemyRanged_Fire.AM_EnemyRanged_Fire" (`self.BulletSpawn`) (`self.Mesh`)))

(fn `UserConstructionScript`
  (`parent.UserConstructionScript`))