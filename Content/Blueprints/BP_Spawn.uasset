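; Enemy spawner that shows a countdown widget, then spawns the next AI pawn at a random point inside the SpawnRange bounds.
; SpawnNextEnemy, run at BeginPlay, resets the countdown, arms spawning and shows the timer widget.
; Tick lowers the countdown per frame, not by delta time, and spawns once it drops below a fixed threshold.
; Spawning disarms the spawner, removes the widget and advances a wrapping EnemyPool index, without re-arming itself.
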(event `self.ReceiveBeginPlay`
  (bind _returnvalue (`|CreateWidget` "/Game/UI/WBP_SpawnTimer.WBP_SpawnTimer_C"))
  (set `self.SpawnTimer` _returnvalue)
  (`self.SpawnNextEnemy`))

(event `self.ReceiveTick`
  (params (DeltaSeconds :type "Float (single-precision)"))
  (if (`self.canSpawn`)
    (bind _output_get (set `self.elapsedTime` (- (`self.elapsedTime`) 1.0)))
    (if (< _output_get 10.0)
      (`self.SpawnEnemy`)
      (set `self.canSpawn` false))))

(event `SpawnEnemy`
  (bind (_origin _boxextent) (`self.GetActorBounds` (`self.spawnRange`) false false))
  (`AIBlueprintHelperLibrary.SpawnAIFromClass` (`|GetArrayItem` (`self.enemyPool`) (`self.spawnIndex`)) null (`KismetMathLibrary.RandomPointInBoundingBox` _origin _boxextent) (struct) true null)
  (set `self.canSpawn` false)
  (`Widget.RemoveFromParent` (`self.SpawnTimer`))
  (bind _result (`/Engine/EditorBlueprintResources/StandardMacros.IncrementInt` (`self.spawnIndex`))
    (:`  `
      (if (> _result 6)
        (set `self.spawnIndex` 0)))))

(fn `SpawnNextEnemy`
  (set `self.elapsedTime` (`self.delayTime`))
  (set `self.canSpawn` true)
  (`UserWidget.AddToViewport` (`self.SpawnTimer`) 0))

(fn `UserConstructionScript`)